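; BP_PatrolRoute is an enemy AI patrol route that exposes the points of its RouteSpline as successive patrol destinations.
; GetSplineWorldPos returns the world location of the spline point at the current PatrolIdx.
; UpdateRouteIdx steps that index by DirectionPatrol and flips the direction at the first and last points, so the route is traversed back and forth rather than looped.
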(event Custom|UpdateRouteIdx
  (bind _output_get (Variables|Default|SetPatrolIdx (+ (Variables|Default|GetPatrolIdx) (Variables|Default|GetDirectionPatrol))))
  (if (== _output_get (- (Spline|GetNumberOfSplinePoints (Variables|Default|GetRouteSpline)) 1))
    (Variables|Default|SetDirectionPatrol -1)
    (elif (== (Variables|Default|GetPatrolIdx) 0)
      (Variables|Default|SetDirectionPatrol 1))))

(fn ConstructionScript)

(fn GetSplineWorldPos
  (return (Spline|GetLocationatSplinePoint (Variables|Default|GetRouteSpline) (Variables|Default|GetPatrolIdx) "World")))