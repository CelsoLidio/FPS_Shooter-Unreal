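; NormalEnemyBP is an AI-controlled rifle enemy that shoots projectiles and exposes a patrol route and walk, sprint or idle speed setting.
; AttackEnemy plays a firing montage, then on completion or interruption spawns BP_EnemyProjectile at BulletSpawn and signals that the shot is done.
; OnDying stops AI movement, disables box collision and plays a slowed hit reaction while a timeline shrinks the mesh before destroying the actor.
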(event Custom|AttackEnemy
  (Animation|Montage|PlayMontage (Variables|Character|GetMesh) "/Game/Assets/Enemies/NormalEnemy/Animations/Montages/AM_firing_rifle.AM_firing_rifle" 0.5
    (:OnCompleted
      _)
    (:OnInterrupted
      _))
  (Game|SpawnActorfromClass "/Game/Blueprint/Weapons/Bullets/BP_EnemyProjectile.BP_EnemyProjectile_C" (Transformation|GetWorldTransform (Variables|Default|GetbulletSpawn)) "Undefined" "MultiplyWithRoot" 0 0)
  (Default|CallOnShootCompleted))

(event EventBeginPlay)

(event Collision|EventActorBeginOverlap
  (params (OtherActor :type Actor%20Object%20Reference)))

(event EventTick
  (params (DeltaSeconds :type Float%20%28single-precision%29)))

(event EventOnDying
  (AI|Navigation|StopMovement (AI|GetAIController self))
  (Collision|SetCollisionEnabled (Variables|Default|GetBox) "NoCollision")
  (Animation|Montage|PlayMontage (Variables|Character|GetMesh) "/Game/Assets/Enemies/NormalEnemy/Animations/Montages/AM_hit_reaction.AM_hit_reaction" 0.1
    (:then
      (bind _newtrack_0 (Timeline|DeathTL PlayFromStart)
        (:Update
          (Transformation|SetRelativeScale3D (Variables|Character|GetMesh) (Math|Vector|Lerp(Vector) "1.000000,1.000000,1.000000" "0.001000,0.001000,0.001000" _newtrack_0)))
        (:Finished
          (Actor|DestroyActor))))))

(fn ConstructionScript)

(fn GetPatrolRoute
  (return (Variables|Default|GetpatrolRoute)))

(fn SetMovementSpeed
  (params (moveSpeedType :type EAIMoveSpeed%20Enum :default "Idle"))
  (bind _output_get (Variables|/Script/Engine.CharacterMovementComponent|SetMaxWalkSpeed (Variables|Character|GetCharacterMovement) (Utilities|Select :Index moveSpeedType :Idle 0.0 :Walking 3e+02 :Sprinting 6e+02)))
  (return _output_get))